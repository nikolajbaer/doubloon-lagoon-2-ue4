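; ShipCharacter is a player-controlled pirate ship character that moves, steers and collects coins.
; Forward/backward input moves it along the control rotation's forward vector, while left/right input turns the controller's yaw.
; A CoinPickedUp event increments the coin count and prints the total.
; Tick fakes ocean swell by pitching the Pirateship component on a sine of game time, with its yaw offset held fixed.
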(event `CoinPickedUp`
  ;[1 1 1] Add Coin
  (bind _output_get (set `self.Coins` (+ (`self.Coins`) 1)))
  (`KismetSystemLibrary.PrintString` (`KismetTextLibrary.Conv_TextToString` (`KismetTextLibrary.Conv_IntToText` _output_get))))

(event `InputAxis|Forward_Backward`
  (params (AxisValue :type "Float (single-precision)"))
  ;[1 1 1] Movement Controls
  (`self.AddMovementInput` (`KismetMathLibrary.GetForwardVector` (`self.GetControlRotation`)) AxisValue))

(event `InputAxis|Left_Right`
  (params (AxisValue :type "Float (single-precision)"))
  ;[1 1 1] Movement Controls
  (`self.AddControllerYawInput` AxisValue))

(event `self.ReceiveTick`
  (params (DeltaSeconds :type "Float (single-precision)"))
  ;[1 1 1] Sway with ocean Swell
  (`SceneComponent.K2_SetRelativeRotation` (`self.pirateship`) (`KismetMathLibrary.MakeRotator` 0.0 (* (`KismetMathLibrary.Sin` (`GameplayStatics.GetTimeSeconds`)) 20.0) -90.0) false false))

(fn `UserConstructionScript`)