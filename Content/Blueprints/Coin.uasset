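; Coin pickup actor that spins in place and is collected when anything overlaps its Cylinder component.
; Overlap disables collision, plays a sound and runs a timeline that lifts the coin, then destroys it and calls the CoinPickedUp dispatcher.
; Spin and rise apply fixed offsets per frame without delta-time scaling, so both depend on frame rate.
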(event `self.Cylinder.OnComponentBeginOverlap`
  (params (OverlappedComponent :type "PrimitiveComponent Object Reference") (OtherActor :type "Actor Object Reference") (OtherComp :type "PrimitiveComponent Object Reference") (OtherBodyIndex :type Integer) (bFromSweep :type Boolean) (SweepResult :type "HitResult Structure (by ref)"))
  ;[1 1 1] Coin Pickup
  (`PrimitiveComponent.SetCollisionEnabled` (`self.Cylinder`) "NoCollision")
  (`GameplayStatics.PlaySoundAtLocation` "/Game/Sounds/ca-ching_ogg.ca-ching_ogg" (`self.K2_GetActorLocation`) (struct) 1.0 1.0 0.0 null null null)
  (`Timeline|Timeline_0`
    (:`Update`
      (`SceneComponent.K2_AddWorldOffset` (`self.DefaultSceneRoot`) (0.0 0.0 10.0) false false))
    (:`Finished`
      (`self.K2_DestroyActor`)
      (`self.CoinPickedUp`))))

(event `self.ReceiveTick`
  (params (DeltaSeconds :type "Float (single-precision)"))
  ;[1 1 1] Coin Spin
  (`SceneComponent.K2_AddLocalRotation` (`self.DefaultSceneRoot`) (struct :`Yaw` 2.0) false false))

(fn `UserConstructionScript`)