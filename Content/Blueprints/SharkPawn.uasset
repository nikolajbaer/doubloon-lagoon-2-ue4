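; SharkPawn is a shark pawn that pitches in reaction to the player's proximity and destroys itself when hit.
; Each tick it measures the distance from its Shark component to player 0's character mesh.
; Inside 100 units it keeps roll and yaw and sets pitch to -45 degrees per unit of closeness, unclamped.
; At or beyond that range it resets the whole actor rotation to zero.
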(event `self.ReceiveHit`
  (params (MyComp :type "PrimitiveComponent Object Reference") (Other :type "Actor Object Reference") (OtherComp :type "PrimitiveComponent Object Reference") (bSelfMoved :type Boolean) (HitLocation :type "Vector Structure") (HitNormal :type "Vector Structure") (NormalImpulse :type "Vector Structure") (Hit :type "HitResult Structure (by ref)"))
  (`self.K2_DestroyActor`))

(event `self.ReceiveTick`
  (params (DeltaSeconds :type "Float (single-precision)"))
  (bind _returnvalue (`KismetMathLibrary.VSize` (- (`SceneComponent.K2_GetComponentLocation` (`Character.Mesh` (`GameplayStatics.GetPlayerCharacter` 0))) (`SceneComponent.K2_GetComponentLocation` (`self.shark`)))))
  (`/Engine/EditorBlueprintResources/StandardMacros.CompareFloat` _returnvalue 100.0
    (:`>`
      (`self.K2_SetActorRotation` (struct) :!label _label))
    (:`==`
      (goto _label))
    (:`<`
      (`self.K2_SetActorRotation` (`KismetMathLibrary.MakeRotator` (.roll (`self.K2_GetActorRotation`)) (* (/ (- 100.0 _returnvalue) 1.0) -45.0) (.yaw (`self.K2_GetActorRotation`)))))))

(fn `UserConstructionScript`)